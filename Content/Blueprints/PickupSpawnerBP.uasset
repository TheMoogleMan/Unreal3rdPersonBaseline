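; PickupSpawnerBP is a spawner actor that creates GuidePickupBP pickups one at a time at a sequence of locations.
; It caches the giBP game instance on BeginPlay, which holds the spawn locations, the current index and a SpawnNext flag.
; Tick polls that flag and, when set, spawns a pickup at the indexed location, clears the flag and increments the index without a bounds check.
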(event Custom|Spawn
  (bind _givar (Variables|Default|GetgiVar))
  (Game|SpawnActorfromClass "/Game/Blueprints/GuidePickupBP.GuidePickupBP_C" (Math|Conversions|ToTransform(Vector) (Utilities|Array|Get(acopy) (Variables|/Game/Blueprints/giBP.giBP_C|GetSpawnLocations _givar) (Variables|/Game/Blueprints/giBP.giBP_C|GetSpawnIndexVar _givar))) "Undefined" 0 0))

(event EventBeginPlay
  (bind _asgi_bp (Utilities|Casting|CastTogiBP (Game|GetGameInstance)))
  (Variables|Default|SetgiVar _asgi_bp))

(event Collision|EventActorBeginOverlap
  (params (OtherActor :type Actor%20Object%20Reference)))

(event EventTick
  (params (DeltaSeconds :type Float%20%28single-precision%29))
  (bind _givar (Variables|Default|GetgiVar))
  (if (Variables|/Game/Blueprints/giBP.giBP_C|GetSpawnNext _givar)
    (CallFunction|Spawn)
    (Variables|/Game/Blueprints/giBP.giBP_C|SetSpawnNext _givar false)
    (bind _result (Math|Integer|IncrementInt (Variables|/Game/Blueprints/giBP.giBP_C|GetSpawnIndexVar _givar))
      (:%20%20
        (Variables|/Game/Blueprints/giBP.giBP_C|SetSpawnIndexVar _givar _result)))))

(fn ConstructionScript)